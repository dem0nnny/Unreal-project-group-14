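; Zombie enemy character that hunts and melee-attacks the first-person player, with a health bar widget that tracks damage until the actor is destroyed.
; Pawn sensing writes pawns seen within a frontal cone to the AI controller's blackboard as TargetActor, and Tick updates InAttackRange from the distance to that target.
; Attack checks facing and range, plays an animation, then applies delayed damage to the player behind a cooldown gate.
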(event `self.ReceiveBeginPlay`
  (bind _aswbp_zombie_health (cast `/Game/Characters/Zombies/WBP_ZombieHealth` (`WidgetComponent.GetUserWidgetObject` (`self.HealthWidget`))))
  (set `self.ZombieHealthUI` _aswbp_zombie_health)
  (set `/Game/Characters/Zombies/WBP_ZombieHealth.HealthPercent` (/ (`self.Health`) (`self.MaxHealth`)) (`self.ZombieHealthUI`)))

(event `TakeDamage`
  (params (Damage :type "Float (double-precision)"))
  (set `self.Health` (- (`self.Health`) Damage))
  (`/Engine/EditorBlueprintResources/StandardMacros.IsValid` (`self.ZombieHealthUI`)
    (:`Is Valid`
      (set `/Game/Characters/Zombies/WBP_ZombieHealth.HealthPercent` (/ (`self.Health`) (`self.MaxHealth`)) (`self.ZombieHealthUI`))
      (if (<= (`self.Health`) 0.0)
        (`self.K2_DestroyActor`)))))

(event `Die`
  (set `self.IsDead` false)
  (`CharacterMovementComponent.DisableMovement` (`self.CharacterMovement`)))

(event `self.PawnSensing.OnSeePawn`
  (params (Pawn :type "Pawn Object Reference"))
  (if (> (`KismetMathLibrary.DotProduct2D` (`KismetMathLibrary.Conv_VectorToVector2D` (`self.GetActorForwardVector`)) (`KismetMathLibrary.NormalSafe2D` (`KismetMathLibrary.Conv_VectorToVector2D` (- (`self.K2_GetActorLocation` Pawn) (`self.K2_GetActorLocation`))))) 0.3)
    (bind _asbp_zombie_aicontroller (cast `/Game/Characters/Zombies/BP_ZombieAIController` (`self.GetController`)))
    (`BlackboardComponent.SetValueAsObject` (`AIController.Blackboard` _asbp_zombie_aicontroller) "TargetActor" Pawn)))

(event `self.ReceiveTick`
  (params (DeltaSeconds :type "Float (single-precision)"))
  (bind _asbp_zombie_aicontroller (cast `/Game/Characters/Zombies/BP_ZombieAIController` (`self.GetController`)))
  (if (!= (`BlackboardComponent.GetValueAsObject` (`AIBlueprintHelperLibrary.GetBlackboard` _asbp_zombie_aicontroller) "TargetActor") null)
    (bind _asactor (cast `Actor` (`BlackboardComponent.GetValueAsObject` (`AIBlueprintHelperLibrary.GetBlackboard` null) "TargetActor")))
    (`BlackboardComponent.SetValueAsBool` (`AIBlueprintHelperLibrary.GetBlackboard` null) "InAttackRange" (<= (`self.GetDistanceTo` _asactor) (`self.AttackRange`)))
    (else
      (`BlackboardComponent.SetValueAsBool` (`AIBlueprintHelperLibrary.GetBlackboard` null) "InAttackRange" false))))

(event `Attack`
  (if (`self.CanAttack`)
    (bind _asbp_first_person_character (cast `/Game/FirstPerson/Blueprints/BP_FirstPersonCharacter` (`GameplayStatics.GetPlayerCharacter` 0)))
    (if (> (`KismetMathLibrary.Dot_VectorVector` (`self.GetActorForwardVector`) (`KismetMathLibrary.Conv_Vector2DToVector` (`KismetMathLibrary.NormalSafe2D` (`KismetMathLibrary.Conv_VectorToVector2D` (- (`self.K2_GetActorLocation` _asbp_first_person_character) (`self.K2_GetActorLocation`)))))) 0.3)
      (if (<= (`self.GetDistanceTo` _asbp_first_person_character) (`self.AttackRange`))
        (set `self.CanAttack` false)
        (`SkeletalMeshComponent.PlayAnimation` (`self.Mesh`) "/Game/Characters/Zombies/zombie_attack.zombie_attack" false)
        (`KismetSystemLibrary.Delay` 0.5)
        (`/Game/FirstPerson/Blueprints/BP_FirstPersonCharacter.TakeDamage_Player` _asbp_first_person_character (`self.AttackDmg`))
        (`KismetSystemLibrary.Delay` (`self.AttackCooldown`))
        (set `self.CanAttack` true)))))

(fn `UserConstructionScript`)